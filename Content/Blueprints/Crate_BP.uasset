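; Crate actor that optionally simulates physics and remembers whether the boxes in the CastleCourtyard level have been moved.
; On BeginPlay, a false Physics flag turns off simulation on its Cube.
; With Physics on in CastleCourtyard, it reads BoxesMoved from Chrome_GI, then either destroys itself or enables simulation.
; In other levels, physics-enabled crates keep the Cube's default setting.
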(event EventBeginPlay
  (bind _cube (Variables|Default|GetCube))
  (if (Variables|Default|Getphysics)
    (bind _returnvalue (Game|GetCurrentLevelName true))
    (if (Utilities|Enum|Equal(Enum) _returnvalue "CastleCourtyard")
      (bind _aschrome_gi (Utilities|Casting|CastToChrome_GI (Game|GetGameInstance)))
      (if (Variables|/Game/Chrome_GI.Chrome_GI_C|GetboxesMoved _aschrome_gi)
        (Actor|DestroyActor)
        (else
          (Physics|SetSimulatePhysics _cube true))))
    (else
      (Physics|SetSimulatePhysics _cube false))))

(event Collision|EventActorBeginOverlap
  (params (OtherActor :type Actor%20Object%20Reference)))

(event EventTick
  (params (DeltaSeconds :type Float%20%28single-precision%29)))

(fn ConstructionScript)