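; Door actor that sends the player to another level when interacted with through the BPIInteract interface event.
; If the sender is the player character, it stores its CameFrom value as CurrentDoor in Chrome_GI, the game instance.
; It then calls MoveLevel with its DoorID on the Chrome_PC player controller and disables the character's movement.
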(event EventBeginPlay)

(event Collision|EventActorBeginOverlap
  (params (OtherActor :type Actor%20Object%20Reference)))

(event EventTick
  (params (DeltaSeconds :type Float%20%28single-precision%29)))

(event EventBPIInteract
  (params (sender :type Actor%20Object%20Reference))
  (bind _asplayer_character_bp (Utilities|Casting|CastToPlayerCharacter_BP sender))
  (bind _aschrome_pc (Utilities|Casting|CastToChrome_PC (Game|GetPlayerController 0)))
  (bind _aschrome_gi (Utilities|Casting|CastToChrome_GI (Game|GetGameInstance)))
  (Variables|/Game/Chrome_GI.Chrome_GI_C|SetcurrentDoor _aschrome_gi (Variables|Default|GetcameFrom))
  (Default|MoveLevel _aschrome_pc (Variables|Default|GetdoorID))
  (bind _asplayer_character_bp_2 (Utilities|Casting|CastToPlayerCharacter_BP _asplayer_character_bp))
  (Pawn|Components|CharacterMovement|DisableMovement (Variables|/Script/Engine.Character|GetCharacterMovement _asplayer_character_bp_2)))

(fn ConstructionScript)