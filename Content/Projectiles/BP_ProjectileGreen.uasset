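; Green projectile Blueprint that leaves a green splat decal where it hits and then destroys itself.
; HitBox overlaps trigger the impact, ignoring PlayerCharacter_BP.
; A small zero-length sphere trace at the projectile's location, with debug drawing left on, supplies the hit normal that orients the temporary decal.
; The construction script only calls its parent.
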(event OnComponentBeginOverlap(HitBox)
  (params (OverlappedComponent :type Primitive%20Component%20Object%20Reference) (OtherActor :type Actor%20Object%20Reference) (OtherComp :type Primitive%20Component%20Object%20Reference) (OtherBodyIndex :type Integer) (bFromSweep :type Boolean) (SweepResult :type Hit%20Result%20Structure%20%28by%20ref%29))
  (bind _returnvalue (Transformation|GetActorLocation))
  (if (not (== OtherActor "/Game/PlayerCharacter_BP.PlayerCharacter_BP"))
    (bind _outhit (Collision|SphereTraceByChannel _returnvalue _returnvalue 3e+01 "TraceTypeQuery1" false 0 "ForDuration"))
    (Rendering|Decal|SpawnDecalatLocation "/Game/Projectiles/Decal_GreenSplat.Decal_GreenSplat" "100.000000,100.000000,100.000000" (Transformation|GetActorLocation) (Math|Rotator|MakeRotfromX (.Normal (Collision|BreakHitResult _outhit))) 3e+01)
    (Actor|DestroyActor)))

(fn ConstructionScript
  (|CallParentFunction))