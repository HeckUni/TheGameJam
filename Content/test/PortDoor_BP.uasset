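; PortDoor_BP is a locked door that opens when a player holding the required key interacts with it.
; The interact event casts the sender to PlayerCharacter_BP and searches its Keys array for a match with KeyNeeded.
; On a match, the DoorMove timeline slides the static mesh by interpolating its relative location from Closed to Open, with no logic to close it again.
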(event EventBeginPlay)

(event Collision|EventActorBeginOverlap
  (params (OtherActor :type Actor%20Object%20Reference)))

(event EventTick
  (params (DeltaSeconds :type Float%20%28single-precision%29)))

(event EventBPIInteract
  (params (sender :type Actor%20Object%20Reference))
  (bind _asplayer_character_bp (Utilities|Casting|CastToPlayerCharacter_BP sender))
  (for _array_element (Variables|/Game/PlayerCharacter_BP.PlayerCharacter_BP_C|Getkeys _asplayer_character_bp)
    (if (== (Variables|Default|GetkeyNeeded) _array_element)
      (bind _alpha (Timeline|DoorMove Play)
        (:Update
          (Transformation|SetRelativeLocation (Variables|Default|GetStaticMesh) (Math|Vector|Lerp(Vector) (Variables|Default|Getclosed) (Variables|Default|GetOpen) _alpha) false false))))))

(fn ConstructionScript)