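; BP_PlatformRed is a platform whose mesh is visible only in the player's red mode.
; After a short delay on BeginPlay, it binds to the player character's red, green and normal mode events, which toggle mesh visibility without changing collision settings.
; A Move event uses a timeline to lerp the mesh between Start and End offsets from Origin, flipping direction on finish, though nothing in this graph initially calls it.
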(event Custom|GreenMode
  (Variables|Default|SetVisibilityMode false)
  (Rendering|SetVisibility (Variables|Debug|GetStaticMeshComponent) (Variables|Default|GetVisibilityMode) false))

(event Custom|RedMode
  (Variables|Default|SetVisibilityMode true)
  (Rendering|SetVisibility (Variables|Debug|GetStaticMeshComponent) (Variables|Default|GetVisibilityMode) false))

(event Custom|NormalMode
  (Variables|Default|SetVisibilityMode false)
  (Rendering|SetVisibility (Variables|Debug|GetStaticMeshComponent) (Variables|Default|GetVisibilityMode) false))

(event Custom|Move
  (bind _origin (Variables|Default|GetOrigin))
  (if (Variables|Default|GetForward)
    (bind _alpha (Timeline|Timeline_0 Play)
      (:Update
        (Transformation|SetWorldLocationAndRotation (Variables|Debug|GetStaticMeshComponent) (Math|Vector|Lerp(Vector) (+ (Variables|Default|GetStart) _origin) (+ (Variables|Default|GetEnd) _origin) _alpha) "0, 0, 0" false false))
      (:Finished
        (Variables|Default|SetForward (not (Variables|Default|GetForward)))
        (CallFunction|Move)))
    (else
      (Timeline|Timeline_0 Reverse))))

(event EventBeginPlay
  (CallFunction|NormalMode)
  (Utilities|FlowControl|Delay 5.0)
  (bind _asplayer_character_bp (Utilities|Casting|CastToPlayerCharacter_BP (Game|GetPlayerCharacter 0)))
  (Variables|Default|SetAs%20Player%20Character%20BP _asplayer_character_bp)
  (EventDispatchers|BindEventtoRedMode (Variables|Default|GetAs%20Player%20Character%20BP) (delegate Custom|RedMode))
  (EventDispatchers|BindEventtoGreenMode (Variables|Default|GetAs%20Player%20Character%20BP) (delegate Custom|GreenMode))
  (EventDispatchers|BindEventtoNormalMode (Variables|Default|GetAs%20Player%20Character%20BP) (delegate Custom|NormalMode)))

(fn ConstructionScript)